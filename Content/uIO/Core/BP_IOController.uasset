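; BP_IOController handles cursor aiming and shooting for the player's BP_IOCharacter.
; On BeginPlay it caches the pawn in a variable named PlayerController, which holds the character despite its name.
; Each tick it yaws the character's sprite toward the visibility-trace hit under the cursor, with fixed roll and a yaw offset.
; The attack input spawns a BP_Bullet at the Bullet component's location with the sprite's rotation, passing the character as owner.
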(event `self.ReceiveBeginPlay`
  (bind _asbp_iocharacter (cast `/Game/uIO/Character/Bp_IOCharacter` (`GameplayStatics.GetPlayerPawn` 0)))
  (set `self.PlayerController` _asbp_iocharacter))

(event `self.ReceiveTick`
  (params (DeltaSeconds :type "Float (single-precision)"))
  (`SceneComponent.K2_SetWorldRotation` (`PaperCharacter.Sprite` (`self.PlayerController`)) (`KismetMathLibrary.MakeRotator` 270.0 0.0 (+ (.yaw (`KismetMathLibrary.FindLookAtRotation` (`self.K2_GetActorLocation` (`self.PlayerController`)) (`.ImpactPoint` (`GameplayStatics.BreakHitResult` (`self.GetHitResultUnderCursorByChannel` "TraceTypeQuery1"))))) 90.0)) false false))

(event `InputAction|attack`
  (params (Key :type "Key Structure"))
  (bind _playercontroller (`self.PlayerController`))
  (:`Pressed`
    (`|SpawnActorFromClass` "/Game/uIO/新建文件夹/BP_Bullet.BP_Bullet_C" (`KismetMathLibrary.MakeTransform` (`SceneComponent.K2_GetComponentLocation` (`/Game/uIO/Character/Bp_IOCharacter.Bullet` _playercontroller)) (`SceneComponent.K2_GetComponentRotation` (`PaperCharacter.Sprite` _playercontroller))) "Undefined" "OverrideRootScale" null _playercontroller null)))

(fn `UserConstructionScript`)