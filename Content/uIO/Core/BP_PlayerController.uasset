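; Player controller for a cursor-aimed character that moves, aims and attacks.
; On BeginPlay it caches the possessed BP_PlayerCharacter in a variable misleadingly named PlayerController.
; Each tick it passes the world point under the cursor, from a complex Visibility trace, to the character's LookAt.
; MoveForward and MoveRight axes add movement along fixed world X and Y, and the attack action calls the character's Attack.
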(event `InputAction|attack`
  (params (Key :type "Key Structure"))
  (:`Pressed`
    (`/Game/uIO/Character/BP_CharacterBase.Attack` (`self.PlayerController`))))

(event `self.ReceiveBeginPlay`
  (bind _asbp_player_character (cast `/Game/uIO/Character/BP_PlayerCharacter` (`GameplayStatics.GetPlayerPawn` 0)))
  (set `self.PlayerController` _asbp_player_character))

(event `self.ReceiveTick`
  (params (DeltaSeconds :type "Float (single-precision)"))
  (`/Game/uIO/Character/BP_CharacterBase.LookAt` (`self.PlayerController`) (`.Location` (`GameplayStatics.BreakHitResult` (`self.GetHitResultUnderCursorByChannel` "TraceTypeQuery1")))))

(event `InputAxis|MoveRight`
  (params (AxisValue :type "Float (single-precision)"))
  (if (!= AxisValue 0.0)
    (`Pawn.AddMovementInput` (`self.PlayerController`) (0.0 1.0 0.0) AxisValue false)))

(event `InputAxis|MoveForward`
  (params (AxisValue :type "Float (single-precision)"))
  (if (!= AxisValue 0.0)
    (`Pawn.AddMovementInput` (`self.PlayerController`) (1.0 0.0 0.0) AxisValue false)))

(fn `UserConstructionScript`)