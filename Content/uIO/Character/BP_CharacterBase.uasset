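; BP_CharacterBase is a character base Blueprint that provides health, damage handling and death.
; On BeginPlay it casts the HpBar component's widget to w_HealthBar and initializes it with a reference to itself.
; AnyDamage subtracts the truncated damage from integer Hp, clamps it between zero and MaxHp, and destroys the actor when Hp reaches zero.
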(event `self.ReceiveBeginPlay`
  (bind _asw_health_bar (cast `/Game/uIO/Hp/w_HealthBar` (`WidgetComponent.GetUserWidgetObject` (`self.HpBar`))))
  (`/Game/uIO/Hp/w_HealthBar.init` _asw_health_bar self))

(event `self.ReceiveAnyDamage`
  (params (Damage :type "Float (single-precision)") (DamageType :type "DamageType Object Reference") (InstigatedBy :type "Controller Object Reference") (DamageCauser :type "Actor Object Reference"))
  (bind _output_get (set `self.Hp` (`KismetMathLibrary.Clamp` (- (`self.Hp`) (`KismetMathLibrary.FTrunc` Damage)) 0 (`self.maxHp`))))
  (if (== _output_get 0)
    (`self.K2_DestroyActor`)))

(fn `UserConstructionScript`)